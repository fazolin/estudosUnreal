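; An actor that pulses its Cube's scale whenever it receives an OSC message.
; BeginPlay creates a listening OSC server on localhost port 1312 and binds its message event.
; Any message, regardless of address or content, restarts ScaleTimeline, whose value drives the cube's uniform relative scale.
; A debug print of the message address and first integer is present but unconnected.
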(event Custom|OnMsgReceived
  (params (Message :type OSC%20Message%20Structure%20%28by%20ref%29) (IPAddress :type String) (Port :type Integer))
  ;[1 1 1] Binding to Any Message
  (bind _value (Timeline|scaleTimeline PlayFromStart)
    (:Update
      (Transformation|SetRelativeScale3D (Variables|Default|GetCube) (Math|Conversions|ToVector(Float) (* _value 1.0))))))

(event EventBeginPlay
  ;[1 1 1] Binding to Any Message
  (bind _returnvalue (Class|OSCManager|CreateOSCServer "127.0.0.1" 1312 false true "" 0))
  (EventDispatchers|AssignOnOscMessageReceived _returnvalue (delegate Custom|OnMsgReceived)))

(fn ConstructionScript)