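; BP_particles1 drives a Niagara particle system's User.Noise parameter from OSC messages.
; On BeginPlay it sets an initial noise value and starts a local OSC server bound to any incoming message.
; Each message's first float is scaled up and written to User.Noise, regardless of address.
; Key 1 plays a Noise timeline that re-runs the same setter; its curve feeds only an unused Lerp.
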(event Custom|OnMsgReceived
  (params (Message :type OSC%20Message%20Structure%20%28by%20ref%29) (IPAddress :type String) (Port :type Integer))
  ;[1 1 1] Binding to Any Message
  (bind _returnvalue (Class|OSCManager|GetOSCMessageAddress Message))
  (bind _returnvalue_2 (Class|OSCManager|GetOSCAddressFullPath _returnvalue))
  (bind _value (Class|OSCManager|GetFloat Message))
  (Development|PrintString (Utilities|String|Append "Address: " _returnvalue_2 "Value: " (Utilities|String|ToString(Float) _value)) false false)
  (Effects|Components|ParticleSystem|SetFloatParameter (Variables|Default|GetNiagara) "User.Noise" (* _value 5e+02)))

(event EventBeginPlay
  (Input|EnableInput (Game|GetPlayerController 0))
  (Effects|Components|ParticleSystem|SetFloatParameter (Variables|Default|GetNiagara) "User.Noise" (Variables|Default|GetParam))
  ;[1 1 1] Binding to Any Message
  (bind _returnvalue (Class|OSCManager|CreateOSCServer "127.0.0.1" 1312 false true "" 0))
  (EventDispatchers|AssignOnOscMessageReceived _returnvalue (delegate Custom|OnMsgReceived)))

(event Input|KeyboardEvents|1
  (params (Key :type Key%20Structure :default "None"))
  (:Pressed
    (bind _value (Timeline|Noise PlayFromStart)
      (:Update
        (Effects|Components|ParticleSystem|SetFloatParameter (Variables|Default|GetNiagara) "User.Noise" (* (stale Custom|OnMsgReceived _value) 5e+02))))))

(fn ConstructionScript)